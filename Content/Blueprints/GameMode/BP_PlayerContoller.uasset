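; Player controller that opens an AGV message widget for the actor clicked under the mouse cursor.
; The Fire input deprojects the cursor and runs a complex Visibility line trace, with its end built from the ray direction alone rather than offset from the start.
; Any hit creates a new BP_AGV_1_WidgetBlueprint in the viewport and passes the actor's first tag to ReadAGVMessages, without checking the actor type.
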(event `InputAction|Fire`
  (params (Key :type "Key Structure"))
  (bind (_worldlocation _worlddirection) (`self.DeprojectMousePositionToWorld` (`GameplayStatics.GetPlayerController` 0)))
  (:`Pressed`
    (bind (_outhit _returnvalue) (`KismetSystemLibrary.LineTraceSingle` _worldlocation (+ _worlddirection (* _worlddirection 100000.0)) "TraceTypeQuery1" true))
    (if _returnvalue
      (if true
        (bind _returnvalue_2 (`|CreateWidget` "/Game/Blueprints/UI/BP_AGV_1_WidgetBlueprint.BP_AGV_1_WidgetBlueprint_C"))
        (`UserWidget.AddToViewport` _returnvalue_2 0)
        (`/Game/Blueprints/UI/BP_AGV_1_WidgetBlueprint.ReadAGVMessages` _returnvalue_2 (`|GetArrayItem` (`Actor.Tags` (`.HitActor` (`GameplayStatics.BreakHitResult` _outhit)))))))))

(fn `UserConstructionScript`)