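; Startup actor for a warehouse AGV visualization that builds the scene from data tables and a WMS server.
; BeginPlay reads server settings, spawns slot-tagged boxes and caches their layout in BP_Instance.
; Chained VaRest GET callbacks then map robot IDs to tagged AGV actors, signal AGVMove, and pass location data to ReadJsonFunc.
; The final tray query attaches stacked boxes to each AGV's occupied tray and fork slots.
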(event `self.ReceiveBeginPlay`
  (for (_ _array_index) (`self.Loopindex`)
    (bind _asbp_instance (cast `/Game/Blueprints/GameInstance/BP_Instance` (`GameplayStatics.GetGameInstance`)))
    (bind _returnvalue (`|GetDataTableRow` "/Game/Blueprints/CVS/configs.configs" "0")
      (:`then`
        (bind (_serverip _port _topic) (break `/Game/Blueprints/BYD/config` _returnvalue))
        (set `/Game/Blueprints/GameInstance/BP_Instance.serverip` _serverip _asbp_instance)
        (set `/Game/Blueprints/GameInstance/BP_Instance.port` _port _asbp_instance)
        (set `/Game/Blueprints/GameInstance/BP_Instance.topic` _topic _asbp_instance)
        (bind _returnvalue_2 (`|GetDataTableRow` "/Game/Blueprints/CVS/chanxian.chanxian" (`KismetStringLibrary.Conv_StringToName` (`KismetStringLibrary.Conv_IntToString` _array_index)))
          (:`then`
            (bind (_startx _starty _endx _endy _dir _rotate _slotcode) (break `/Game/Blueprints/BYD/SlotData` _returnvalue_2))
            (bind _returnvalue_3 (`KismetStringLibrary.Conv_StringToDouble` (`KismetStringLibrary.Concat_StrStr` "-" (`KismetStringLibrary.Conv_DoubleToString` _startx))))
            (bind _returnvalue_4 (`|SpawnActorFromClass` "/Game/Blueprints/BYD/BP_Box_01.BP_Box_01_C" (`KismetMathLibrary.MakeTransform` (`KismetMathLibrary.MakeVector` _returnvalue_3 _starty 70.0) (`KismetMathLibrary.MakeRotator` 0.0 0.0 (`KismetMathLibrary.Conv_IntToDouble` _rotate))) "Undefined" "OverrideRootScale" null null))
            (bind _tags (`Actor.Tags` _returnvalue_4))
            (`KismetArrayLibrary.Array_Add` _tags (`KismetStringLibrary.Conv_StringToName` _slotcode))
            (set `Actor.Tags` _tags _returnvalue_4)
            (bind _asbp_instance_2 (cast `/Game/Blueprints/GameInstance/BP_Instance` (`GameplayStatics.GetGameInstance`)))
            (`KismetArrayLibrary.Array_Add` (`/Game/Blueprints/GameInstance/BP_Instance.StartX` _asbp_instance_2) _returnvalue_3)
            (`KismetArrayLibrary.Array_Add` (`/Game/Blueprints/GameInstance/BP_Instance.StartY` _asbp_instance_2) _starty)
            (`KismetArrayLibrary.Array_Add` (`/Game/Blueprints/GameInstance/BP_Instance.EndX` _asbp_instance_2) (`KismetStringLibrary.Conv_StringToDouble` (`KismetStringLibrary.Concat_StrStr` "-" (`KismetStringLibrary.Conv_DoubleToString` _endx))))
            (`KismetArrayLibrary.Array_Add` (`/Game/Blueprints/GameInstance/BP_Instance.EndY` _asbp_instance_2) _endy)
            (`KismetArrayLibrary.Array_Add` (`/Game/Blueprints/GameInstance/BP_Instance.Dir` _asbp_instance_2) _dir)
            (`BlueprintMapLibrary.Map_Add` (`/Game/Blueprints/GameInstance/BP_Instance.Slot2index` _asbp_instance_2) _slotcode _array_index)
            (bind _boxes (`/Game/Blueprints/GameInstance/BP_Instance.Boxes` _asbp_instance_2))
            (`KismetArrayLibrary.Array_Add` _boxes _returnvalue_4))))))
  (for _array_element _boxes
    (`self.SetActorHiddenInGame` _array_element false))
  (bind _returnvalue_5 (`KismetStringLibrary.Concat_StrStr` "http://" _serverip ":" (`KismetStringLibrary.Conv_IntToString` _port)))
  (set `/Game/Blueprints/GameInstance/BP_Instance.HttpUrl` _returnvalue_5 _asbp_instance)
  (`VaRestSubsystem.CallURL` (subsystem `VaRestSubsystem`) (`KismetStringLibrary.Concat_StrStr` _returnvalue_5 "/ess-api/wms/robotcode") "GET" "x_www_form_urlencoded_url" null (delegate `Callback`)))

(event `Callback`
  (params (Request :type "VaRestRequestJSON Object Reference"))
  (bind _returnvalue (`VaRestRequestJSON.GetResponseObject` Request))
  (bind _returnvalue_2 (subsystem `VaRestSubsystem`))
  (if (== (`VaRestJsonObject.GetIntegerField` _returnvalue "code") 200)
    (for _array_element (`VaRestJsonObject.GetObjectArrayField` _returnvalue "data")
      (bind _devicemap (`/Game/Blueprints/GameInstance/BP_Instance.devicemap` (stale `self.ReceiveBeginPlay` _asbp_instance)))
      (bind _returnvalue_3 (`VaRestJsonObject.GetStringField` _array_element "devicecode"))
      (if (`.ReturnValue` (`BlueprintMapLibrary.Map_Find` _devicemap _returnvalue_3))
        (`BlueprintMapLibrary.Map_Remove` _devicemap _returnvalue_3)
        (`BlueprintMapLibrary.Map_Add` _devicemap _returnvalue_3 (`VaRestJsonObject.GetStringField` _array_element "deviceid"))))
    (bind _keys (`BlueprintMapLibrary.Map_Keys` _devicemap))
    (for _array_element_2 _keys
      _)
    (for (_array_element_3 _array_index) (`/Game/Blueprints/GameInstance/BP_Instance.N60` (stale `self.ReceiveBeginPlay` _asbp_instance))
      (bind _returnvalue_4 (`KismetStringLibrary.Concat_StrStr` "kubot-" (`KismetStringLibrary.Conv_IntToString` _array_element_3)))
      (bind _outactors (`GameplayStatics.GetAllActorsOfClassWithTag` "/Game/HaiKeSiKang/model/AGVMode/AGV_A42T.AGV_A42T_C" (`KismetStringLibrary.Conv_StringToName` _returnvalue_4)))
      (bind _output (`|GetArrayItem` _outactors))
      (`BlueprintMapLibrary.Map_Add` (`/Game/Blueprints/GameInstance/BP_Instance.AGVActorMap` (stale `self.ReceiveBeginPlay` _asbp_instance)) _returnvalue_4 _output)
      (bind (_returnvalue_x _returnvalue_y) (`KismetMathLibrary.BreakVector` (`self.K2_GetActorLocation` _output)))
      (`KismetSystemLibrary.PrintString` (`KismetStringLibrary.Conv_DoubleToString` _returnvalue_x))
      (`KismetArrayLibrary.Array_Add` (`/Game/Blueprints/GameInstance/BP_Instance.XoffArray` (stale `self.ReceiveBeginPlay` _asbp_instance)) _returnvalue_x)
      (`KismetArrayLibrary.Array_Add` (`/Game/Blueprints/GameInstance/BP_Instance.YoffArray` (stale `self.ReceiveBeginPlay` _asbp_instance)) _returnvalue_y)
      (`BlueprintMapLibrary.Map_Add` (`/Game/Blueprints/GameInstance/BP_Instance.DeviceID2Index` (stale `self.ReceiveBeginPlay` _asbp_instance)) _returnvalue_4 _array_index)
      (`BlueprintMapLibrary.Map_Add` (`/Game/Blueprints/GameInstance/BP_Instance.Kubotinfo` (stale `self.ReceiveBeginPlay` _asbp_instance)) _returnvalue_4))
    (bind _returnvalue_5 (`GameplayStatics.GetActorOfClass` "/Game/Blueprints/BYD/AGVMove.AGVMove_C"))
    (bind _asagvmove (cast `/Game/Blueprints/BYD/AGVMove` _returnvalue_5))
    (`/Game/Blueprints/BYD/AGVMove.InitEnd` _asagvmove)
    (bind _returnvalue_6 (`VaRestSubsystem.ConstructVaRestJsonObject` _returnvalue_2))
    (`VaRestSubsystem.CallURL` _returnvalue_2 (`KismetStringLibrary.Concat_StrStr` (`/Game/Blueprints/GameInstance/BP_Instance.HttpUrl` (stale `self.ReceiveBeginPlay` _asbp_instance)) "/ess-api/wms/locationQuery2") "GET" "x_www_form_urlencoded_url" _returnvalue_6 (delegate `Call`))))

(event `Call`
  (params (Request :type "VaRestRequestJSON Object Reference"))
  (bind _returnvalue (`VaRestRequestJSON.GetResponseContentAsString` Request true))
  (`self.ReadJsonFunc` _returnvalue)
  (`VaRestSubsystem.CallURL` (subsystem `VaRestSubsystem`) (`KismetStringLibrary.Concat_StrStr` (`/Game/Blueprints/GameInstance/BP_Instance.HttpUrl` (stale `self.ReceiveBeginPlay` _asbp_instance)) "/ess-api/wms/agvtrays") "GET" "x_www_form_urlencoded_url" null (delegate `Trays`)))

(event `Trays`
  (params (Request :type "VaRestRequestJSON Object Reference"))
  (bind _values (`BlueprintMapLibrary.Map_Values` (`/Game/Blueprints/GameInstance/BP_Instance.devicemap` (stale `self.ReceiveBeginPlay` _asbp_instance))))
  (for _array_element _values
    (`|ExecutionSequence`
      (:`then_0`
        (bind _returnvalue (`VaRestJsonObject.GetObjectField` (`VaRestRequestJSON.GetResponseObject` Request) _array_element))
        (if (`KismetStringLibrary.NotEqual_StrStr` (`VaRestJsonObject.GetStringField` _returnvalue "0"))
          (bind _returnvalue_2 (`|SpawnActorFromClass` "/Game/Blueprints/BYD/BP_Box_01.BP_Box_01_C" (`KismetMathLibrary.MakeTransform` (0.0 0.0 0.0)) "Undefined" "OverrideRootScale" null null))
          (bind _value (`BlueprintMapLibrary.Map_Find` (`/Game/Blueprints/GameInstance/BP_Instance.AGVActorMap` (stale `self.ReceiveBeginPlay` _asbp_instance)) _array_element))
          (`self.K2_AttachToActor` _returnvalue_2 _value "None" "KeepRelative" "KeepRelative" "KeepRelative" true)
          (`SceneComponent.K2_SetRelativeLocation` (`Actor.RootComponent` _returnvalue_2) (-50.0 0.0 75.0) false false)
          (`KismetSystemLibrary.PrintString` "设置背篓0")))
      (:`then_1`
        (if (`KismetStringLibrary.NotEqual_StrStr` (`VaRestJsonObject.GetStringField` _returnvalue "1"))
          (bind _returnvalue_3 (`|SpawnActorFromClass` "/Game/Blueprints/BYD/BP_Box_01.BP_Box_01_C" (`KismetMathLibrary.MakeTransform` (0.0 0.0 0.0)) "Undefined" "OverrideRootScale" null null))
          (`self.K2_AttachToActor` _returnvalue_3 _value "None" "KeepRelative" "KeepRelative" "KeepRelative" true)
          (`SceneComponent.K2_SetRelativeLocation` (`Actor.RootComponent` _returnvalue_3) (-50.0 0.0 120.0) false false)
          (`KismetSystemLibrary.PrintString` "设置背篓1")))
      (:`then_2`
        (if (`KismetStringLibrary.NotEqual_StrStr` (`VaRestJsonObject.GetStringField` _returnvalue "2"))
          (bind _returnvalue_4 (`|SpawnActorFromClass` "/Game/Blueprints/BYD/BP_Box_01.BP_Box_01_C" (`KismetMathLibrary.MakeTransform` (0.0 0.0 0.0)) "Undefined" "OverrideRootScale" null null))
          (`self.K2_AttachToActor` _returnvalue_4 _value "None" "KeepRelative" "KeepRelative" "KeepRelative" true)
          (`SceneComponent.K2_SetRelativeLocation` (`Actor.RootComponent` _returnvalue_4) (-50.0 0.0 165.0) false false)
          (`KismetSystemLibrary.PrintString` "设置背篓2")))
      (:`then_3`
        (if (`KismetStringLibrary.NotEqual_StrStr` (`VaRestJsonObject.GetStringField` _returnvalue "3"))
          (bind _returnvalue_5 (`|SpawnActorFromClass` "/Game/Blueprints/BYD/BP_Box_01.BP_Box_01_C" (`KismetMathLibrary.MakeTransform` (0.0 0.0 0.0)) "Undefined" "OverrideRootScale" null null))
          (`self.K2_AttachToActor` _returnvalue_5 _value "None" "KeepRelative" "KeepRelative" "KeepRelative" true)
          (`SceneComponent.K2_SetRelativeLocation` (`Actor.RootComponent` _returnvalue_5) (-50.0 0.0 210.0) false false)
          (`KismetSystemLibrary.PrintString` "设置背篓3")))
      (:`then_4`
        (if (`KismetStringLibrary.NotEqual_StrStr` (`VaRestJsonObject.GetStringField` _returnvalue "4"))
          (bind _returnvalue_6 (`|SpawnActorFromClass` "/Game/Blueprints/BYD/BP_Box_01.BP_Box_01_C" (`KismetMathLibrary.MakeTransform` (0.0 0.0 0.0)) "Undefined" "OverrideRootScale" null null))
          (`self.K2_AttachToActor` _returnvalue_6 _value "None" "KeepRelative" "KeepRelative" "KeepRelative" true)
          (`SceneComponent.K2_SetRelativeLocation` (`Actor.RootComponent` _returnvalue_6) (-50.0 0.0 255.0) false false)
          (`KismetSystemLibrary.PrintString` "设置背篓4")))
      (:`then_5`
        (if (`KismetStringLibrary.NotEqual_StrStr` (`VaRestJsonObject.GetStringField` _returnvalue "5"))
          (bind _returnvalue_7 (`|SpawnActorFromClass` "/Game/Blueprints/BYD/BP_Box_01.BP_Box_01_C" (`KismetMathLibrary.MakeTransform` (0.0 0.0 0.0)) "Undefined" "OverrideRootScale" null null))
          (`self.K2_AttachToActor` _returnvalue_7 _value "None" "KeepRelative" "KeepRelative" "KeepRelative" true)
          (`SceneComponent.K2_SetRelativeLocation` (`Actor.RootComponent` _returnvalue_7) (-50.0 0.0 300.0) false false)
          (`KismetSystemLibrary.PrintString` "设置背篓5")))
      (:`then_6`
        (if (`KismetStringLibrary.NotEqual_StrStr` (`VaRestJsonObject.GetStringField` _returnvalue "6"))
          (bind _returnvalue_8 (`|SpawnActorFromClass` "/Game/Blueprints/BYD/BP_Box_01.BP_Box_01_C" (`KismetMathLibrary.MakeTransform` (0.0 0.0 0.0)) "Undefined" "OverrideRootScale" null null))
          (`self.K2_AttachToActor` _returnvalue_8 _value "None" "KeepRelative" "KeepRelative" "KeepRelative" true)
          (`SceneComponent.K2_SetRelativeLocation` (`Actor.RootComponent` _returnvalue_8) (-50.0 0.0 345.0) false false)
          (`KismetSystemLibrary.PrintString` "设置背篓6")))
      (:`then_7`
        (if (`KismetStringLibrary.NotEqual_StrStr` (`VaRestJsonObject.GetStringField` _returnvalue "64"))
          (bind _returnvalue_9 (`|SpawnActorFromClass` "/Game/Blueprints/BYD/BP_Box_01.BP_Box_01_C" (`KismetMathLibrary.MakeTransform` (0.0 0.0 0.0)) "Undefined" "OverrideRootScale" null null))
          (`self.K2_AttachToActor` _returnvalue_9 _value "None" "KeepRelative" "KeepRelative" "KeepRelative" true)
          (`SceneComponent.K2_SetRelativeLocation` (`Actor.RootComponent` _returnvalue_9) (-50.0 0.0 390.0) false false)
          (`KismetSystemLibrary.PrintString` "设置货叉64"))))))

(fn `UserConstructionScript`)