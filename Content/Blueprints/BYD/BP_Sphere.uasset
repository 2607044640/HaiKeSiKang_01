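; BP_Sphere is an actor that travels along a supplied spline, with controls to start, stop and reverse it.
; Move plays a timeline whose alpha maps to distance along the spline, setting location and rotation from Local-space spline values.
; Move overrides its Speed input with a zero play rate, so motion waits for Start.
; Start, Stop and NewTime set fixed forward, zero or negative rates and print Chinese status messages.
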(event `Move`
  (params (Line :type "/Game/Blueprints/BYD/BP_Productionline_Spline_01 Object Reference") (Speed :type "Float (double-precision)"))
  (bind _spline (`/Game/Blueprints/BYD/BP_Productionline_Spline_01.Spline` Line))
  (`TimelineComponent.SetPlayRate` (`self.Time1`) Speed)
  (`TimelineComponent.SetPlayRate` (`self.Time1`) 0.0)
  (bind (_direction _alpha) (`Timeline|Time1` :!via `PlayFromStart`)
    (:`Update`
      (bind _returnvalue (`KismetMathLibrary.Lerp` 0.0 (`SplineComponent.GetSplineLength` _spline) _alpha))
      (`self.K2_SetActorLocationAndRotation` (`SplineComponent.GetLocationAtDistanceAlongSpline` _spline _returnvalue "Local") (`SplineComponent.GetRotationAtDistanceAlongSpline` _spline _returnvalue "Local")))))

(event `Stop`
  (`TimelineComponent.SetPlayRate` (`self.Time1`) 0.0)
  (`KismetSystemLibrary.PrintString` "停止"))

(event `Start`
  (`TimelineComponent.SetPlayRate` (`self.Time1`) 0.03)
  (`KismetSystemLibrary.PrintString` "开始"))

(event `NewTime`
  (`TimelineComponent.SetPlayRate` (`self.Time1`) -0.03)
  (`KismetSystemLibrary.PrintString` "按照线路返回"))

(fn `UserConstructionScript`)