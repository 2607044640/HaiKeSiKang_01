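; Drives the AGV actors in the scene from device data stored in BP_Instance, mirroring position, fork pose and status.
; InitEnd starts a fast looping timer that steps each AGV one unit toward its target, Y then X, snapping when target X trails by over 100.
; On arrival it applies body yaw and fork extension, rotation and height.
; A field split from Kubotinfo shows the red indicator for ERROR, otherwise green.
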(event `InitEnd`
  (bind _asbp_instance (cast `/Game/Blueprints/GameInstance/BP_Instance` (`GameplayStatics.GetGameInstance`)))
  (`KismetSystemLibrary.K2_SetTimerDelegate` (delegate `AGVMove`) 0.00625 true))

(event `self.ReceiveBeginPlay`)

(event `AGVMove`
  (bind _values (`BlueprintMapLibrary.Map_Values` (`/Game/Blueprints/GameInstance/BP_Instance.devicemap` (stale `InitEnd` _asbp_instance))))
  (for _array_element _values
    (`|ExecutionSequence`
      (:`then_0`
        (bind _value (`BlueprintMapLibrary.Map_Find` (`/Game/Blueprints/GameInstance/BP_Instance.DeviceID2Index` (stale `InitEnd` _asbp_instance)) _array_element))
        (bind _output (`|GetArrayItem` (`/Game/Blueprints/GameInstance/BP_Instance.XoffArray` (stale `InitEnd` _asbp_instance)) _value))
        (bind _value_2 (`BlueprintMapLibrary.Map_Find` (`/Game/Blueprints/GameInstance/BP_Instance.AGVActorMap` (stale `InitEnd` _asbp_instance)) _array_element))
        (bind (_returnvalue_x _returnvalue_y) (`KismetMathLibrary.BreakVector` (`self.K2_GetActorLocation` _value_2)))
        (if (< (- _output _returnvalue_x) -100.0)
          (set `self.Xoff` _output)
          (bind _output_2 (`|GetArrayItem` (`/Game/Blueprints/GameInstance/BP_Instance.YoffArray` (stale `InitEnd` _asbp_instance)) _value))
          (set `self.Yoff` _output_2)
          (`self.K2_SetActorLocation` _value_2 (`KismetMathLibrary.MakeVector` (`self.Xoff`) (`self.Yoff`)) false false))
        (if (`KismetMathLibrary.NearlyEqual_FloatFloat` _returnvalue_y _output_2 1.0)
          (if (`KismetMathLibrary.NearlyEqual_FloatFloat` _returnvalue_x _output 1.0)
            (`self.K2_SetActorRotation` _value_2 (`KismetMathLibrary.MakeRotator` 0.0 0.0 (`|GetArrayItem` (`/Game/Blueprints/GameInstance/BP_Instance.AGVRotate` (stale `InitEnd` _asbp_instance)) _value)) false)
            (`|ExecutionSequence`
              (:`then_0`
                (if (> (`|GetArrayItem` (`/Game/Blueprints/GameInstance/BP_Instance.ForkLong` (stale `InitEnd` _asbp_instance)) _value) 0.0)
                  (bind _agv02_line5290 (`/Game/HaiKeSiKang/model/AGVMode/AGV_A42T.agv02_Line5290` _value_2))
                  (`SceneComponent.K2_SetRelativeLocation` _agv02_line5290 (0.0 120.0 0.0) false false)
                  (bind _agv02_line5291 (`/Game/HaiKeSiKang/model/AGVMode/AGV_A42T.agv02_Line5291` _value_2))
                  (`SceneComponent.K2_SetRelativeLocation` _agv02_line5291 (0.0 70.0 0.0) false false)
                  (else
                    (`SceneComponent.K2_SetRelativeLocation` _agv02_line5290 (0.0 60.0 0.0) false false)
                    (`SceneComponent.K2_SetRelativeLocation` _agv02_line5291 (0.0 0.0 0.0) false false))))
              (:`then_1`
                (bind _staticmesh (`/Game/HaiKeSiKang/model/AGVMode/AGV_A42T.StaticMesh` _value_2))
                (`SceneComponent.K2_SetRelativeRotation` _staticmesh (`KismetMathLibrary.MakeRotator` 0.0 0.0 (`|GetArrayItem` (`/Game/Blueprints/GameInstance/BP_Instance.ForkRotate` (stale `InitEnd` _asbp_instance)) _value)) false false)
                (bind _output_3 (`|GetArrayItem` (`/Game/Blueprints/GameInstance/BP_Instance.ForkHigh` (stale `InitEnd` _asbp_instance)) _value))
                (if (== _output_3 0.0)
                  (set `self.ForkHight` 15.0)
                  (else
                    (set `self.ForkHight` _output_3)))
                (`SceneComponent.K2_SetRelativeLocation` _staticmesh (`KismetMathLibrary.MakeVector` 0.0 -53.0 (`self.ForkHight`)) false false) ; 货叉高度
              ))
            (elif (> _output _returnvalue_x)
              (bind _result (`/Engine/EditorBlueprintResources/StandardMacros.IncrementFloat` _returnvalue_x)
                (:`  `
                  (`self.K2_SetActorLocation` _value_2 (`KismetMathLibrary.MakeVector` _result _returnvalue_y) false false)))
              (else
                (bind _result_2 (`/Engine/EditorBlueprintResources/StandardMacros.DecrementFloat` _returnvalue_x)
                  (:`  `
                    (`self.K2_SetActorLocation` _value_2 (`KismetMathLibrary.MakeVector` _result_2 _returnvalue_y) false false))))))
          (elif (> _output_2 _returnvalue_y)
            (bind _result_3 (`/Engine/EditorBlueprintResources/StandardMacros.IncrementFloat` _returnvalue_y)
              (:`  `
                (`self.K2_SetActorLocation` _value_2 (`KismetMathLibrary.MakeVector` _returnvalue_x _result_3) false false)))
            (else
              (bind _result_4 (`/Engine/EditorBlueprintResources/StandardMacros.DecrementFloat` _returnvalue_y)
                (:`  `
                  (`self.K2_SetActorLocation` _value_2 (`KismetMathLibrary.MakeVector` _returnvalue_x _result_4) false false)))))))
      (:`then_1`
        (bind _value_3 (`BlueprintMapLibrary.Map_Find` (`/Game/Blueprints/GameInstance/BP_Instance.Kubotinfo` (stale `InitEnd` _asbp_instance)) _array_element))
        (if (`KismetStringLibrary.NotEqual_StrStr` _value_3)
          (bind _lefts (`KismetStringLibrary.Split` (`.RightS` (`KismetStringLibrary.Split` (`.RightS` (`KismetStringLibrary.Split` (`.RightS` (`KismetStringLibrary.Split` (`.RightS` (`KismetStringLibrary.Split` _value_3 ",")) ",")) ",")) ",")) ","))
          (if (`KismetStringLibrary.EqualEqual_StrStr` _lefts "ERROR")
            (bind _gr (`/Game/HaiKeSiKang/model/AGVMode/AGV_A42T.Gr` _value_2))
            (`SceneComponent.SetHiddenInGame` _gr true false)
            (bind _red (`/Game/HaiKeSiKang/model/AGVMode/AGV_A42T.Red` _value_2))
            (`SceneComponent.SetHiddenInGame` _red false false)
            (elif (`KismetStringLibrary.EqualEqual_StrStr` _lefts "EXECUTING")
              (`SceneComponent.SetHiddenInGame` _red true false)
              (`SceneComponent.SetHiddenInGame` _gr false false)
              (else
                (`SceneComponent.SetHiddenInGame` _red true false)
                (`SceneComponent.SetHiddenInGame` _gr false false)))))))))

(fn `UserConstructionScript`)