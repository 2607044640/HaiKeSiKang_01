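; Production-line controller that animates boxes from slot status held in BP_Instance, and adds a ChatUI widget on BeginPlay.
; A looping 0.02-second timer compares Status with PreStatus per slot to detect changes.
; Activation either spawns a BP_Box_02, tagging it and logging any container's position, or shows an existing box.
; Active existing boxes step toward their end point, X before Y; deactivation hides and resets the box to its start.
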(event `Box01`
  ;[1 1 1] 注释
  (`self.SetActorHiddenInGame` (`|GetArrayItem` (`self.Boxes`) 1) false))

(event `Box02`
  ;[1 1 1] 注释
  (`self.SetActorHiddenInGame` (`|GetArrayItem` (`self.Boxes`)) false))

(event `self.ReceiveTick`
  (params (DeltaSeconds :type "Float (single-precision)"))
  ;[1 1 1] 注释
)

(event `self.ReceiveBeginPlay`
  ;[1 1 1] 注释
  ;;[1 1 1] 开始
  (bind _returnvalue (`|CreateWidget` "/BPMqtt/ChatUI.ChatUI_C"))
  (bind _output_get (set `self.ChatUI` _returnvalue))
  (`UserWidget.AddToViewport` _output_get 0)
  (`KismetSystemLibrary.K2_SetTimerDelegate` (delegate `Get01Productionline`) 0.02 true))

(event `Get01Productionline`
  ;[1 1 1] 注释
  ;;[1 1 1] 开始
  (bind _asbp_instance (cast `/Game/Blueprints/GameInstance/BP_Instance` (`GameplayStatics.GetGameInstance`)))
  (bind _prestatus (`/Game/Blueprints/GameInstance/BP_Instance.PreStatus` _asbp_instance))
  (for (_array_element _array_index) _prestatus
    (bind _asbp_instance_2 (cast `/Game/Blueprints/GameInstance/BP_Instance` (`GameplayStatics.GetGameInstance`)))
    (bind _output (`|GetArrayItem` (`/Game/Blueprints/GameInstance/BP_Instance.Status` _asbp_instance) _array_index))
    (if (not (and (== _array_element 0) (== _output 0)))
      (bind _returnvalue (== _output 1))
      (if (and (== _array_element 0) _returnvalue)
        (bind _value (`BlueprintMapLibrary.Map_Find` (`self.IsCreate`) _array_index))
        (if _value
          (bind (_value_2 _returnvalue_2) (`BlueprintMapLibrary.Map_Find` (`/Game/Blueprints/GameInstance/BP_Instance.SlotBoxRotation` _asbp_instance) (`KismetStringLibrary.Conv_IntToString` _array_index)))
          (if _returnvalue_2
            (set `self.ZRotation` (`KismetMathLibrary.Conv_IntToDouble` _value_2))
            (else
              (set `self.ZRotation` 0.0)))
          (bind _output_2 (`|GetArrayItem` (`/Game/Blueprints/GameInstance/BP_Instance.StartX` _asbp_instance) _array_index))
          (bind _output_3 (`|GetArrayItem` (`/Game/Blueprints/GameInstance/BP_Instance.StartY` _asbp_instance) _array_index))
          (bind _returnvalue_3 (`|SpawnActorFromClass` "/Game/Blueprints/BYD/BP_Box_02.BP_Box_02_C" (`KismetMathLibrary.MakeTransform` (`KismetMathLibrary.MakeVector` _output_2 _output_3 70.0) (`KismetMathLibrary.MakeRotator` 0.0 0.0 (`self.ZRotation`))) "Undefined" "OverrideRootScale" null null))
          (`KismetArrayLibrary.Array_Set` _prestatus _array_index _output)
          (bind _output_4 (`|GetArrayItem` (`/Game/Blueprints/GameInstance/BP_Instance.slotContainers` _asbp_instance) _array_index))
          (if (not (`KismetStringLibrary.EqualEqual_StrStr` _output_4))
            (bind _tags (`Actor.Tags` _returnvalue_3))
            (`KismetArrayLibrary.Array_Add` _tags (`KismetStringLibrary.Conv_StringToName` _output_4))
            (set `Actor.Tags` _tags _returnvalue_3)
            (bind (_returnvalue_x _returnvalue_y _returnvalue_z) (`KismetMathLibrary.BreakVector` (`self.K2_GetActorLocation` _returnvalue_3)))
            (`BlueprintMapLibrary.Map_Add` (`/Game/Blueprints/GameInstance/BP_Instance.ContainerInfo` _asbp_instance) _output_4 (`KismetStringLibrary.Concat_StrStr` (`KismetStringLibrary.Conv_DoubleToString` _returnvalue_x) "," (`KismetStringLibrary.Conv_DoubleToString` _returnvalue_y) "," (`KismetStringLibrary.Conv_DoubleToString` _returnvalue_z))))
          (else
            (bind _output_5 (`|GetArrayItem` (`/Game/Blueprints/GameInstance/BP_Instance.Boxes` _asbp_instance_2) _array_index))
            (`self.SetActorHiddenInGame` _output_5 false)
            ;;[1 1 1] 位移
            (`KismetSystemLibrary.PrintString` (`KismetStringLibrary.Concat_StrStr` (`KismetStringLibrary.Conv_IntToString` _array_index) "索引：" "箱子显示"))
            (`KismetArrayLibrary.Array_Set` _prestatus _array_index _output)))
        (else
          (bind _returnvalue_4 (== _array_element 1))
          (if (and _returnvalue _returnvalue_4)
            (if (not _value)
              (bind (_returnvalue_x_2 _returnvalue_y_2) (`KismetMathLibrary.BreakVector` (`self.K2_GetActorLocation` _output_5)))
              (bind _output_6 (`|GetArrayItem` (`/Game/Blueprints/GameInstance/BP_Instance.EndX` _asbp_instance) _array_index))
              (if (`KismetMathLibrary.NearlyEqual_FloatFloat` _returnvalue_x_2 _output_6 5.0)
                (set `self.SetBox1X` _returnvalue_x_2)
                (bind _output_7 (`|GetArrayItem` (`/Game/Blueprints/GameInstance/BP_Instance.EndY` _asbp_instance) _array_index))
                (if (not (`KismetMathLibrary.NearlyEqual_FloatFloat` _returnvalue_y_2 _output_7 5.0))
                  (if (> _returnvalue_y_2 _output_7)
                    (set `self.SetBox1Y` (- _returnvalue_y_2 1.0))
                    (else
                      (set `self.SetBox1Y` (+ _returnvalue_y_2 1.0))))
                  (`self.K2_SetActorLocation` _output_5 (`KismetMathLibrary.MakeVector` (`self.SetBox1X`) (`self.SetBox1Y`) 70.0) false false :!label _label)
                  (`KismetArrayLibrary.Array_Set` _prestatus _array_index _output))
                (else
                  (set `self.SetBox1Y` _returnvalue_y_2)
                  (if (> _returnvalue_x_2 _output_6)
                    (set `self.SetBox1X` (- _returnvalue_x_2 1.0))
                    (goto _label)
                    (else
                      (set `self.SetBox1X` (+ _returnvalue_x_2 1.0))
                      (goto _label))))))
            (elif (and _returnvalue_4 (== _output 0))
              (`self.SetActorHiddenInGame` _output_5 true)
              (`self.K2_SetActorLocation` _output_5 (`KismetMathLibrary.MakeVector` _output_2 _output_3 70.0) false false)
              (`KismetArrayLibrary.Array_Set` _prestatus _array_index _output))))))))

(fn `UserConstructionScript`)